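; Demon AI character that toggles a blindfolded state and mirrors it to its AI controller's Blackboard.
; Three seconds after BeginPlay, it caches its AIC_demon controller for Blackboard access.
; TriggerBlindfold uses a FlipFlop to set or clear the blindfolded and player keys, keeping the local Blindfold flag in sync.
; Tick prints that flag on screen as debug output.
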(event EventBeginPlay
  (Utilities|FlowControl|Delay 3.0)
  (bind _asaic_demon (Utilities|Casting|CastToAIC_demon (Pawn|GetController)))
  (Variables|Default|SetAs%20AIC%20Demon _asaic_demon))

(event EventTriggerBlindfold
  (bind _returnvalue (Utilities|Name|MakeLiteralName "player"))
  (bind _returnvalue_2 (Utilities|Name|MakeLiteralName "blindfolded"))
  (bind _as_aic_demon (Variables|Default|GetAs%20AIC%20Demon))
  (bind _as_aic_demon_2 (Variables|Default|GetAs%20AIC%20Demon))
  (bind _returnvalue_3 (AI|GetBlackboard _as_aic_demon))
  (bind _returnvalue_4 (AI|GetBlackboard _as_aic_demon_2))
  (Utilities|FlowControl|FlipFlop
    (:A
      (AI|Components|Blackboard|SetValueasBool _returnvalue_4 _returnvalue_2 true)
      (Variables|Default|Setblindfold true)
      (AI|Components|Blackboard|SetValueasObject _returnvalue_3 _returnvalue (Game|GetPlayerCharacter 0)))
    (:B
      (AI|Components|Blackboard|ClearValue _returnvalue_4 _returnvalue_2)
      (Variables|Default|Setblindfold false)
      (AI|Components|Blackboard|ClearValue _returnvalue_3 _returnvalue))))

(event EventTick
  (params (DeltaSeconds :type Float%20%28single-precision%29))
  (Development|PrintString (Utilities|String|ToString(Boolean) (Variables|Default|Getblindfold)) true true "(R=0.000000,G=0.660000,B=1.000000,A=1.000000)" 0.0))

(fn ConstructionScript)