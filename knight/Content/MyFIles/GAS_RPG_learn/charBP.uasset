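; Player character Blueprint from a Gameplay Ability System RPG learning project, testing leveled stats with heal and damage abilities.
; BeginPlay applies GE_PlayerStats at level 1 and grants GA_Heal and GA_Damage, which left and right mouse buttons trigger by tag for damage and heal respectively.
; F increments Level and applies GE_PlayerStats again at that level.
; Tick prints an attribute pair and Level as a debug readout.
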(event EventBeginPlay
  (GameplayEffects|ApplyGameplayEffectToSelf :self (Variables|Default|GetAbilitySystemComponent) :GameplayEffectClass "/Game/MyFIles/GAS_RPG_learn/GE_PlayerStats.GE_PlayerStats_C" :Level 1.0)
  (GameplayAbilities|GiveAbility (Variables|Default|GetAbilitySystemComponent) "/Game/MyFIles/GAS_RPG_learn/GA_Heal.GA_Heal_C" 0 -1)
  (GameplayAbilities|GiveAbility (Variables|Default|GetAbilitySystemComponent) "/Game/MyFIles/GAS_RPG_learn/GA_Damage.GA_Damage_C" 0 -1))

(event EventTick
  (params (DeltaSeconds :type Float%20%28single-precision%29))
  (bind _abilitysystemcomponent (Variables|Default|GetAbilitySystemComponent))
  (Development|PrintString (Utilities|String|Append (Utilities|String|ToString(Float) (.ReturnValue (Ability|Attribute|GetFloatAttributefromAbilitySystemComponent _abilitysystemcomponent "(AttributeName=\"CurrentHealth\",Attribute=/Script/knight.RPGAttributeSet:CurrentHealth,AttributeOwner=\"/Script/CoreUObject.Class'/Script/knight.RPGAttributeSet'\")"))) " / " (Utilities|String|ToString(Float) (.ReturnValue (Ability|Attribute|GetFloatAttributefromAbilitySystemComponent _abilitysystemcomponent "(AttributeName=\"MaxHealth\",Attribute=/Script/knight.RPGAttributeSet:MaxHealth,AttributeOwner=\"/Script/CoreUObject.Class'/Script/knight.RPGAttributeSet'\")")))) true true "(R=0.000000,G=0.660000,B=1.000000,A=1.000000)" 0.0)
  (Development|PrintString (Utilities|String|Append "Level : " (Utilities|String|ToString(Float) (Variables|Default|Getlevel))) true true "(R=0.000000,G=0.660000,B=1.000000,A=1.000000)" 0.0))

(event Input|KeyboardEvents|F
  (params (Key :type Key%20Structure :default "None"))
  (:Pressed
    (bind _output_get (Variables|Default|Setlevel (+ (Variables|Default|Getlevel) 1.0)))
    (GameplayEffects|ApplyGameplayEffectToSelf :self (Variables|Default|GetAbilitySystemComponent) :GameplayEffectClass "/Game/MyFIles/GAS_RPG_learn/GE_PlayerStats.GE_PlayerStats_C" :Level _output_get)))

(event Input|MouseEvents|LeftMouseButton
  (params (Key :type Key%20Structure :default "None"))
  (:Pressed
    (Abilities|TryActivateAbilitiesbyTag (Variables|Default|GetAbilitySystemComponent) (Variables|Default|GetdamageTag) true)))

(event Input|MouseEvents|RightMouseButton
  (params (Key :type Key%20Structure :default "None"))
  (:Pressed
    (Abilities|TryActivateAbilitiesbyTag (Variables|Default|GetAbilitySystemComponent) (Variables|Default|GethealTag) true)))

(fn ConstructionScript)