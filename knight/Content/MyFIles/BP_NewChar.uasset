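; BP_NewChar is a playable character Blueprint with Enhanced Input movement, look and jump.
; BeginPlay adds the default mapping context through the BP_FirstPersonPlayerController's input subsystem.
; For Gameplay Ability System combat, handlePunch sends a Weapon.Hit gameplay event to the instigator, with the character itself as target data.
; Punch and health-change events print debug text, the latter showing current health.
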(event Custom|punchEvent
  (Development|PrintString "Punch action " true true "(R=0.000000,G=0.660000,B=1.000000,A=1.000000)" 11.0))

(event Custom|handlePunch
  (bind _returnvalue (Game|GetInstigator))
  (bind _self self)
  (Ability|SendGameplayEventtoActor _returnvalue "(TagName=\"Weapon.Hit\")" (Utilities|Struct|MakeGameplayEventData "(TagName=\"\")" _returnvalue _self 0 0 "()" "(GameplayTags=)" "(GameplayTags=)" 0.0 (Ability|TargetData|AbilityTargetDatafromActor _self))))

(event Input|EnhancedActionEvents|EnhancedInputActionIA_Move
  (params (ActionValue :type Vector%202D%20Structure) (ElapsedSeconds :type Float%20%28double-precision%29) (TriggeredSeconds :type Float%20%28double-precision%29) (InputAction :type Input%20Action%20Object%20Reference :default "/Game/ThirdPerson/Input/Actions/IA_Move.IA_Move"))
  (bind (_x _y) (Math|Vector2D|BreakVector2D ActionValue))
  (Pawn|Input|AddMovementInput (Transformation|GetActorForwardVector) _y false)
  (Pawn|Input|AddMovementInput (Transformation|GetActorRightVector) _x false))

(event Input|EnhancedActionEvents|EnhancedInputActionIA_Look
  (params (ActionValue :type Vector%202D%20Structure) (ElapsedSeconds :type Float%20%28double-precision%29) (TriggeredSeconds :type Float%20%28double-precision%29) (InputAction :type Input%20Action%20Object%20Reference :default "/Game/ThirdPerson/Input/Actions/IA_Look.IA_Look"))
  (bind (_x _y) (Math|Vector2D|BreakVector2D ActionValue))
  (Pawn|Input|AddControllerYawInput _x)
  (Pawn|Input|AddControllerPitchInput _y))

(event Input|EnhancedActionEvents|EnhancedInputActionIA_Jump
  (params (ActionValue :type Boolean) (ElapsedSeconds :type Float%20%28double-precision%29) (TriggeredSeconds :type Float%20%28double-precision%29) (InputAction :type Input%20Action%20Object%20Reference :default "/Game/ThirdPerson/Input/Actions/IA_Jump.IA_Jump"))
  (:Triggered
    (Character|Jump))
  (:Canceled
    (Character|StopJumping :!label _label))
  (:Completed
    (goto _label)))

(event EventBeginPlay
  (bind _asbp_first_person_player_controller (Utilities|Casting|CastToBP_FirstPersonPlayerController (Game|GetPlayerController 0)))
  (Utilities|IsValid (PlayerController|LocalPlayerSubsystems|GetEnhancedInputLocalPlayerSubsystem _asbp_first_person_player_controller)
    (:Is%20Valid
      (Input|AddMappingContext (PlayerController|LocalPlayerSubsystems|GetEnhancedInputLocalPlayerSubsystem _asbp_first_person_player_controller) "/Game/ThirdPerson/Input/IMC_Default.IMC_Default" 0 "(bIgnoreAllPressedKeysUntilRelease=True,bForceImmediately=False,bNotifyUserSettings=False)"))))

(event EventOnHealthChanged
  (params (DeltaValue :type Float%20%28single-precision%29) (EventTags :type Gameplay%20Tag%20Container%20Structure%20%28by%20ref%29))
  (bind _returnvalue (Class|MyCharacter|GetHealth))
  (Development|PrintString (Utilities|String|ToString(Float) _returnvalue)))

(event Input|ActionEvents|InputActionPunch
  (params (Key :type Key%20Structure)))

(fn ConstructionScript)